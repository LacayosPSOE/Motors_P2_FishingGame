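; Fishing bobber actor that takes over the camera, removes third-person input, and runs a catch sequence.
; Its first hit starts a random timer, apparently leading to the hooked event, which spawns a fish and plays a timeline bob.
; That opens a Stardew-style minigame widget with caught and broken-tension callbacks.
; Both return the camera and clean up; a catch shows the fish's weight, while a break destroys the fish.
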(event Custom|OnHookedFish
  (Variables|Default|SetFishHooked true)
  (bind _returnvalue (Game|SpawnActorfromClass "/Game/Blueprints/Fish/FishBlueprint.FishBlueprint_C" (Transformation|GetActorTransform) "Undefined" "MultiplyWithRoot" 0 0))
  (Variables|Default|SetFish _returnvalue)
  (bind _bob (Timeline|Bobbing%20Animation Play)
    (:Update
      (Transformation|SetRelativeLocation (Variables|Default|GetCylinder) (* "0.000000,0.000000,20.000000" _bob) false false)
      (Utilities|FlowControl|DoOnce false
        (:Completed
          (bind _returnvalue_2 (UserInterface|CreateWidget "/Game/Blueprints/StardewMinigame.StardewMinigame_C"))
          (UserInterface|Viewport|AddtoViewport _returnvalue_2 0)
          (bind _output_get (Variables|Default|SetAs%20Stardew%20Minigame _returnvalue_2))
          (EventDispatchers|BindEventtoOnFishCaught _output_get (EventDispatchers|CreateEvent :!event Custom|Fish%20caught))
          (EventDispatchers|BindEventtoOnBreakTension _output_get (EventDispatchers|CreateEvent :!event Custom|BreakTension)))))))

(event Custom|BreakTension
  (Game|Player|SetViewTargetwithBlend (Game|GetPlayerController 0) (Game|GetPlayerCharacter 0) 0.5 "VTBlend_Linear" 0.0 false)
  (Utilities|FlowControl|Delay 0.6)
  (Actor|DestroyActor (Variables|Default|GetFish))
  (Widget|RemovefromParent (Variables|Default|GetAs%20Stardew%20Minigame))
  (Actor|DestroyActor))

(event Custom|Fish%20caught
  (bind _returnvalue (UserInterface|CreateWidget "/Game/Blueprints/CaughtFish.CaughtFish_C" 0 (Variables|/Game/Blueprints/Fish/FishBlueprint.FishBlueprint_C|GetWeight (Variables|Default|GetFish))))
  (UserInterface|Viewport|AddtoViewport _returnvalue 0)
  (Game|Player|SetViewTargetwithBlend (Game|GetPlayerController 0) (Game|GetPlayerCharacter 0) 0.5 "VTBlend_Linear" 0.0 false)
  (Utilities|FlowControl|Delay 0.6)
  (Widget|RemovefromParent (Variables|Default|GetAs%20Stardew%20Minigame))
  (Actor|DestroyActor))

(event EventBeginPlay
  (bind _returnvalue (Game|GetPlayerController 0))
  (Game|Player|SetViewTargetwithBlend _returnvalue self 0.5 "VTBlend_Linear" 0.0 false)
  (Input|RemoveMappingContext (PlayerController|LocalPlayerSubsystems|GetEnhancedInputLocalPlayerSubsystem _returnvalue) "/Game/Input/InputMapping_ThirdPerson.InputMapping_ThirdPerson" "(bIgnoreAllPressedKeysUntilRelease=True,bForceImmediately=False,bNotifyUserSettings=False)"))

(event Collision|EventHit
  (params (MyComp :type Primitive%20Component%20Object%20Reference) (Other :type Actor%20Object%20Reference) (OtherComp :type Primitive%20Component%20Object%20Reference) (bSelfMoved :type Boolean) (HitLocation :type Vector :default "0, 0, 0") (HitNormal :type Vector :default "0, 0, 0") (NormalImpulse :type Vector :default "0, 0, 0") (Hit :type Hit%20Result%20Structure%20%28by%20ref%29))
  (Utilities|FlowControl|DoOnce false
    (:Completed
      (Utilities|Time|SetTimerbyEvent (EventDispatchers|CreateEvent :!event Custom|OnHookedFish) (Math|Random|RandomFloatinRange 3.0 6.0)))))

(fn ConstructionScript)